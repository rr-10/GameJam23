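; BP_FollowCam is a side-scroller camera actor that finds BP_SideScrollPlayer on BeginPlay and becomes player 0's view target.
; Each Tick it copies the player character's Y and Z, holding X at OffsetX, with no smoothing.
; The construction script pre-positions it from ToFollow using a fixed Z or dead-zone offset, both ignored at runtime.
; That script feeds target X into camera Y and finally writes look-at yaw into location Z.
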(event EventBeginPlay
  (bind _returnvalue (Actor|GetActorOfClass "/Game/Blueprints/BP_SideScrollPlayer.BP_SideScrollPlayer_C"))
  (Variables|Default|SetToFollow _returnvalue)
  (Game|Player|SetViewTargetwithBlend (Game|GetPlayerController 0) self 0.0 "VTBlend_Linear" 0.0 false))

(event Collision|EventActorBeginOverlap
  (params (OtherActor :type Actor%20Object%20Reference)))

(event EventTick
  (params (DeltaSeconds :type Float%20%28single-precision%29))
  (CallFunction|GetYAxis)
  (CallFunction|GetZAxis)
  (Transformation|SetActorLocation (Math|Vector|MakeVector (Variables|Default|GetOffsetX) (Variables|Default|GetCameraY) (Variables|Default|GetCameraZ)) false false))

(fn ConstructionScript
  (bind _tofollow (Variables|Default|GetToFollow))
  (bind _returnvalue (Transformation|GetActorLocation _tofollow))
  (Utilities|IsValid _tofollow
    (:Is%20Valid
      (bind _output_get (Variables|Default|SetCameraY (.x _returnvalue)))
      (if (!= (Variables|Default|GetFixedZValue) 0.0)
        (Variables|Default|SetCameraZ (Variables|Default|GetFixedZValue))
        (else
          (bind _output_get_2 (Variables|Default|SetCameraZ (+ (.z _returnvalue) (Variables|Default|GetDeadZoneZ))))))
      (Transformation|SetActorLocation (Math|Vector|MakeVector (Variables|Default|GetOffsetX) _output_get _output_get_2) false false)
      (Transformation|SetActorLocation (Math|Vector|MakeVector 0.0 0.0 (.yaw (Math|Rotator|FindLookatRotation (Transformation|GetActorLocation) (Transformation|GetActorLocation (Variables|Default|GetToFollow))))) false false))))

(fn GetYAxis
  (Variables|Default|SetCameraY (.y (Transformation|GetActorLocation (Game|GetPlayerCharacter 0)))))

(fn GetZAxis
  (Variables|Default|SetCameraZ (.z (Transformation|GetActorLocation (Game|GetPlayerCharacter 0)))))